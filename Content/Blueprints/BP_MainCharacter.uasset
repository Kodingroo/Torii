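; BP_MainCharacter is the player character Blueprint, driving a flipbook sprite and a looping Wings component.
; Wings starts hidden at an offset, and each Tick shows it while the player character's JumpCounter exceeds one, suggesting a multi-jump effect.
; Tick reads that counter by casting player character 0 to MainCharacter.
; SetAnimationState selects the sprite's flipbook by state, but always sets Idle, ignoring its AnimState input.
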(event EventBeginPlay
  (Rendering|SetVisibility (Variables|Default|GetWings) false false)
  (Components|Timeline|SetLooping (Variables|Default|GetWings) true)
  (Transformation|SetRelativeLocation (Variables|Default|GetWings) "0,-20.000000,10.000000" false false))

(event Collision|EventActorBeginOverlap
  (params (OtherActor :type Actor%20Object%20Reference)))

(event EventTick
  (params (DeltaSeconds :type Float%20%28single-precision%29))
  (bind _asmain_character (Utilities|Casting|CastToMainCharacter (Game|GetPlayerCharacter 0)))
  (Rendering|SetVisibility (Variables|Default|GetWings) (> (Variables|/Script/Torii.MainCharacter|GetJumpCounter _asmain_character) 1) false)
  (Audio|Components|Audio|Play (Variables|Default|GetWings)))

(fn ConstructionScript)

(fn SetAnimationState
  (params (Anim%20State :type AnimationStates%20Enum :default "NewEnumerator0"))
  (Variables|Default|SetCurrentAnimationState "NewEnumerator0")
  (Sprite|SetFlipbook (Variables|Default|GetSprite) (Utilities|Select :Index (Variables|Default|GetCurrentAnimationState) :NewEnumerator0 (Variables|Default|GetIdle) :NewEnumerator1 (Variables|Default|GetRun) :NewEnumerator2 (Variables|Default|GetJumping) :NewEnumerator3 (Variables|Default|GetLanding) :NewEnumerator4 (Variables|Default|GetHit)))
  (return))